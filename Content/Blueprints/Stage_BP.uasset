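; Stage actor for a minesweeper-style game that builds the tile board, picks mines and tracks play time.
; Pressing F runs InitialGame, which spawns a rotated grid of Tile_BP actors, each given its index and stage reference.
; Mine indices come from shuffling ShuffleIndex, which is not filled here, with the count scaled by difficulty.
; GameStart starts a timeline-driven timer text once; DeleteAllTile and GameReset are empty stubs.
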(event `GameTimeStart`
  ;[1 1 1] Game Time Start 발생 시 게임 타이머를 시작하며, Game Time Stop시 시간을 정지함
  (bind (_direction _playtime) (`Timeline|GameTimeLine` :!label _label)
    (:`Update`
      (bind _output_get (set `self.PlayTime` _playtime))
      (set `self.PlayTimeText` (`KismetTextLibrary.Conv_IntToText` (`KismetMathLibrary.FFloor` _output_get))))))

(event `self.ReceiveBeginPlay`
  (`self.EnableInput` (`GameplayStatics.GetPlayerController` 0)))

(event `GameTimeStop`
  ;[1 1 1] Game Time Start 발생 시 게임 타이머를 시작하며, Game Time Stop시 시간을 정지함
  (goto _label :!via `Stop`))

(event `Key|F`
  (params (Key :type "Key Structure"))
  (:`Pressed`
    (`self.InitialGame`)))

(fn `DeleteAllTile`)

(fn `GameReset`)

(fn `GameStart`
  (if (not (`self.GameStarted`))
    (set `self.GameStarted` true)
    (`self.GameTimeStart`)))

(fn `GetGridLocation`
  (params (Index :type Integer))
  (returns (Location :type "Vector2D Structure"))
  (return (`KismetMathLibrary.MakeVector2D` (* (* (/ Index (`self.GridX`)) (`self.GridMod`)) -1.0) (* (mod Index (`self.GridX`)) (`self.GridMod`)))))

(fn `InitialGame`
  (bind _shuffleindex (`self.ShuffleIndex`))
  (bind _rotation (.rotation (`self.GetTransform`)))
  (`self.DeleteAllTile`)
  (set `self.MaxTile` (* (`self.GridX`) (`self.GridY`)))
  (set `self.PlayTime` 0.0)
  (for _index (range (`self.MaxTile`))
    ;[1 1 1] 스테이지 로케이션에 그리드 위치를 더함
    (bind _location (`self.GetGridLocation` _index))
    (bind (_x _y) (`KismetMathLibrary.BreakVector2D` _location))
    (bind _returnvalue (`|SpawnActorFromClass` "/Game/Blueprints/Tile_BP.Tile_BP_C" (`KismetMathLibrary.MakeTransform` (+ (.location (`self.GetTransform`)) (`KismetMathLibrary.GreaterGreater_VectorRotator` (`KismetMathLibrary.MakeVector` _x _y -47.0) _rotation)) _rotation) "Undefined" "OverrideRootScale" null self _index null))
    (bind _returnvalue_2 (`KismetArrayLibrary.Array_Add` (`self.AllTile`) _returnvalue))
    (`KismetSystemLibrary.PrintString` (`KismetStringLibrary.Conv_IntToString` _returnvalue_2)))
  ;[1 1 1] 랜덤 지뢰 선택 로직
  (bind _output_get (set `self.MaxMineCount` (`KismetMathLibrary.FFloor` (* (`self.MaxTile`) (`self.Defficult`)))))
  (`KismetArrayLibrary.Array_Shuffle` _shuffleindex)
  (for (_array_element _array_index) _shuffleindex
    (if (== _array_index _output_get)
      (break)
      (else
        (`KismetArrayLibrary.Array_Add` (`self.MineIndex`) _array_element)
        (set `self.MineCount` (+ (`self.MineCount`) 1))))))

(fn `UserConstructionScript`)