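; Minesweeper grid tile actor that can be flagged, opened, or end the game through its stage reference when it is a mine.
; InitNearTiles gathers up to eight neighbours from the stage's tile list, rejecting out-of-range and row-wrapping indices, then counts adjacent mines for the text label.
; TileOpen hides the cover, reveals the text and recursively opens neighbours when that count is zero.
; SetFlag toggles flag visibility and tile status.
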(event `self.ReceiveBeginPlay`)

(event `/Game/Interfaces/TileInterface.DoAction`)

(event `/Game/Interfaces/TileInterface.ProjectileHit`)

(event `/Game/Interfaces/TileInterface.WhenLookUp`)

(event `SetFlag`
  (bind _status (`self.Status`))
  (bind _flag (`self.Flag`))
  ;[1 1 1] 깃발을 꽂습니다. - Veiled, QMark 상태일 경우 깃발을 꽂습니다. / Flaged상태일 경우 깃발을 제거합니다.
  (if (or (`|EnumEquality` _status "NewEnumerator0") (`|EnumEquality` _status "NewEnumerator3"))
    (`SceneComponent.SetVisibility` _flag true false)
    (set `self.Status` "NewEnumerator2")
    (elif (`|EnumEquality` (`self.Status`) "NewEnumerator2")
      (`SceneComponent.SetVisibility` _flag false false)
      (set `self.Status` "NewEnumerator0"))))

(event `TileCheck`)

(event `HideCover`
  ;[1 1 1] 타일의 커버를 제거합니다. / 제거하면서 지뢰 글자를 렌더링 합니다.
  (`SceneComponent.SetVisibility` (`self.Cover`) false false)
  (`SceneComponent.SetHiddenInGame` (`self.TextRender`) false false))

(event `OpenNearTiles`
  (for (_array_element _array_index) (`/Game/Blueprints/Stage_BP.AllTile` (`self.StageReference`)) :!label _label
    (for _array_element_2 (`self.NearTiles`)
      (if (== (`/Game/Blueprints/Tile_BP.TileIndex` _array_element_2) _array_index)
        (`self.TileOpen` _array_element)
        (goto _label :!via `Break`)))))

(event `TileOpen`
  (bind _status (`self.Status`))
  ;[1 1 1] 타일 오픈 - 타일의 상태가 Veiled, QMark 일 경우 타일을 오픈합니다./지뢰일경우 게임오버 됩니다.
  (if (or (`|EnumEquality` _status "NewEnumerator0") (`|EnumEquality` _status "NewEnumerator3"))
    (`self.HideCover`)
    (set `self.Status` "NewEnumerator1")
    (if (`self.IsMine`)
      (`ActorComponent.Activate` (`self.ParticleSystem`) false)
      (`/Game/Blueprints/Stage_BP.GameOver` (`self.StageReference`))
      (elif (== (`self.NearMine`) 0)
        (`self.OpenNearTiles`)))))

(event `InitNearTiles`
  (`KismetArrayLibrary.Array_Clear` (`self.NearTiles`))
  (`self.AvailableNearTileIndexCheckAndAdd` (- (- (`self.TileIndex`) (`self.GridX`)) 1))
  (`self.AvailableNearTileIndexCheckAndAdd` (- (`self.TileIndex`) (`self.GridX`)))
  (`self.AvailableNearTileIndexCheckAndAdd` (+ (- (`self.TileIndex`) (`self.GridX`)) 1))
  (`self.AvailableNearTileIndexCheckAndAdd` (- (`self.TileIndex`) 1))
  (`self.AvailableNearTileIndexCheckAndAdd` (+ (`self.TileIndex`) 1))
  (`self.AvailableNearTileIndexCheckAndAdd` (- (+ (`self.TileIndex`) (`self.GridX`)) 1))
  (`self.AvailableNearTileIndexCheckAndAdd` (+ (`self.TileIndex`) (`self.GridX`)))
  (`self.AvailableNearTileIndexCheckAndAdd` (+ (+ (`self.TileIndex`) (`self.GridX`)) 1))
  (set `self.NearMine` 0)
  (for _array_element (`self.NearTiles`)
    (if (`/Game/Blueprints/Tile_BP.IsMine` _array_element)
      (bind _output_get (set `self.NearMine` (+ (`self.NearMine`) 1)))
      (if (`self.IsMine`)
        (`TextRenderComponent.K2_SetText` (`self.TextRender`) "%")
        (elif (not (== _output_get 0))
          (`TextRenderComponent.K2_SetText` (`self.TextRender`) (`KismetTextLibrary.Conv_IntToText` _output_get)))))))

(fn `AvailableNearTileIndexCheckAndAdd`
  (params (NearIndex :type Integer))
  (locals (LocalNearIndex :type Integer))
  (bind _gridx (`self.GridX`))
  (bind _tileindex (`self.TileIndex`))
  (bind _localnearindex (`local.LocalNearIndex`))
  (bind _gridx_2 (`self.GridX`))
  (bind _returnvalue (mod _localnearindex _gridx))
  (set `local.LocalNearIndex` NearIndex)
  (if (not (or (not (and (>= _localnearindex 0) (< _localnearindex (* _gridx (`self.GridY`))))) (and (== _returnvalue (- _gridx 1)) (== (mod _tileindex _gridx_2) 0)) (and (== _returnvalue 0) (== (mod _tileindex _gridx_2) (- _gridx_2 1)))))
    (for _array_element (`/Game/Blueprints/Stage_BP.AllTile` (`self.StageReference`))
      (if (== (`local.LocalNearIndex`) (`/Game/Blueprints/Tile_BP.TileIndex` _array_element))
        (`KismetArrayLibrary.Array_Add` (`self.NearTiles`) _array_element)))))

(fn `UserConstructionScript`
  (bind _stagereference (`self.StageReference`))
  (set `self.GridX` (`/Game/Blueprints/Stage_BP.GridX` _stagereference))
  (set `self.GridY` (`/Game/Blueprints/Stage_BP.GridY` _stagereference))
  (`TextRenderComponent.K2_SetText` (`self.TextRender`) (`self.TileText`)))